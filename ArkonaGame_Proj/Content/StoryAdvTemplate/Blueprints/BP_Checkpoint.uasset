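; BP_Checkpoint is a checkpoint trigger that saves the game when the player pawn overlaps it.
; It enables itself two seconds after BeginPlay, leaving time for the Game Controller to destroy it first.
; On the first valid overlap, it adds its object name to BP_GameController's CollectedOrTriggered list and calls SaveGame on that controller.
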(event `self.ReceiveBeginPlay`
  ;[1 1 1] Enable if not destroyed by Game Controller
  (`KismetSystemLibrary.Delay` 2.0)
  (set `self.Enabled?` true))

(event `self.Trigger.OnComponentBeginOverlap`
  (params (OverlappedComponent :type "PrimitiveComponent Object Reference") (OtherActor :type "Actor Object Reference") (OtherComp :type "PrimitiveComponent Object Reference") (OtherBodyIndex :type Integer) (bFromSweep :type Boolean) (SweepResult :type "HitResult Structure (by ref)"))
  ;[1 1 1] Save Game on Overlap and Destroy Actor
  (if (`self.Enabled?`)
    (if (== (`ActorComponent.GetOwner` OtherComp) (`GameplayStatics.GetPlayerPawn` 0))
      (`/Engine/EditorBlueprintResources/StandardMacros.DoOnce` false
        (:`Completed`
          (bind _outactors (`GameplayStatics.GetAllActorsOfClass` "/Game/StoryAdvTemplate/Blueprints/BP_GameController.BP_GameController_C"))
          (bind _output (`|GetArrayItem` _outactors))
          (`KismetArrayLibrary.Array_AddUnique` (`/Game/StoryAdvTemplate/Blueprints/BP_GameController.CollectedOrTriggered` _output) (`KismetSystemLibrary.GetObjectName` self))
          (`/Game/StoryAdvTemplate/Blueprints/BP_GameController.SaveGame` _output))))))

(fn `UserConstructionScript`
  (`parent.UserConstructionScript`))